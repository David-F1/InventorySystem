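; Inventory component that stores picked-up items as an array of item structs and shows them in an inventory widget.
; AddToInventory merges stackable items by name within their max quantity, otherwise appends them, then refreshes the widget and destroys the item actor.
; A weapon check destroys same-name duplicates of one object type without adding them.
; IA_Inventory opens the widget with UI-only input and a mouse cursor, with no closing logic here.
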(event Input|EnhancedActionEvents|EnhancedInputActionIA_Inventory
  (params (ActionValue :type Boolean) (ElapsedSeconds :type Float%20%28double-precision%29) (TriggeredSeconds :type Float%20%28double-precision%29) (InputAction :type Input%20Action%20Object%20Reference :default "/Game/Input/Actions/IA_Inventory.IA_Inventory"))
  (bind _returnvalue (Game|GetPlayerController 0))
  (bind _inventoryuiref (Variables|Default|GetInventoryUIRef))
  (bind _inventoryuiref_2 (Variables|Default|GetInventoryUIRef))
  ;[0.15 0.15 0.15 0.5] Inventory Action
  (if (not (UserInterface|Viewport|IsinViewport _inventoryuiref_2))
    (UserInterface|Viewport|AddtoViewport _inventoryuiref_2 0)
    (Variables|/Script/Engine.PlayerController|SetbShowMouseCursor _returnvalue true)
    (Input|SetInputModeUIOnly _returnvalue _inventoryuiref "DoNotLock" false)
    (Variables|/Script/UMG.UserWidget|SetbIsFocusable _inventoryuiref true)))

(event EventBeginPlay
  ;[0.15 0.15 0.15 0.5] BeginPlay
  (bind _returnvalue (UserInterface|CreateWidget "/Game/Inventory/Blueprint/W_InventoryUI.W_InventoryUI_C"))
  (bind _output_get (Variables|Default|SetInventoryUIRef _returnvalue))
  (Default|UpdateInventory _output_get self))

(fn AddtoInventory
  (params (BaseItemActor :type BP%20Master-Interactible%20Object%20Reference))
  (bind _inventoryuiref (Variables|Default|GetInventoryUIRef))
  (LocalVariables|SetL%20ItemInteracted BaseItemActor)
  ;[0.15 0.15 0.15 0.5] Verifying if Item should be stacked or not
  (bind (_array_element _array_index) (Utilities|Array|ForEachLoopwithBreak (Variables|Default|GetBaseItem) :!label _label)
    (:LoopBody
      (Utilities|IsValid BaseItemActor
        (:Is%20Valid
          (Variables|Default|SetCurrentIndex _array_index)
          (bind _canadd_ (CallFunction|ShouldStackItem? _array_element (Variables|/Game/BP_Master-Interactible.BP_Master-Interactible_C|GetBaseItemStruct (LocalVariables|GetL%20ItemInteracted))))
          (if _canadd_
            (goto _label Break)))))
    (:Completed
      (if (Variables|Default|GetFoundAndStackable?)
        ;[0.15 0.15 0.15 0.5] Icrementing Item Amount for Stackable Objects
        (Utilities|Array|SetArrayElem (Variables|Default|GetBaseItem) (Variables|Default|GetCurrentIndex) (Utilities|Struct|MakeS_BaseObject (.InventoryItem? (Utilities|Struct|BreakS_BaseObject (Variables|/Game/BP_Master-Interactible.BP_Master-Interactible_C|GetBaseItemStruct (LocalVariables|GetL%20ItemInteracted)))) (.Name (Utilities|Struct|BreakS_BaseObject (Variables|/Game/BP_Master-Interactible.BP_Master-Interactible_C|GetBaseItemStruct (LocalVariables|GetL%20ItemInteracted)))) (.Description (Utilities|Struct|BreakS_BaseObject (Variables|/Game/BP_Master-Interactible.BP_Master-Interactible_C|GetBaseItemStruct (LocalVariables|GetL%20ItemInteracted)))) (.ObjectType (Utilities|Struct|BreakS_BaseObject (Variables|/Game/BP_Master-Interactible.BP_Master-Interactible_C|GetBaseItemStruct (LocalVariables|GetL%20ItemInteracted)))) (.Mesh (Utilities|Struct|BreakS_BaseObject (Variables|/Game/BP_Master-Interactible.BP_Master-Interactible_C|GetBaseItemStruct (LocalVariables|GetL%20ItemInteracted)))) (.Icon (Utilities|Struct|BreakS_BaseObject (Variables|/Game/BP_Master-Interactible.BP_Master-Interactible_C|GetBaseItemStruct (LocalVariables|GetL%20ItemInteracted)))) (.Stackable? (Utilities|Struct|BreakS_BaseObject (Variables|/Game/BP_Master-Interactible.BP_Master-Interactible_C|GetBaseItemStruct (LocalVariables|GetL%20ItemInteracted)))) (Variables|Default|GetNewItemAmount) (.MaxQuantity (Utilities|Struct|BreakS_BaseObject (Variables|/Game/BP_Master-Interactible.BP_Master-Interactible_C|GetBaseItemStruct (LocalVariables|GetL%20ItemInteracted)))) (.Weight (Utilities|Struct|BreakS_BaseObject (Variables|/Game/BP_Master-Interactible.BP_Master-Interactible_C|GetBaseItemStruct (LocalVariables|GetL%20ItemInteracted))))))
        ;[0.15 0.15 0.15 0.5] Updating inventory widget
        (Utilities|IsValid _inventoryuiref :!label _label_2
          (:Is%20Valid
            (Variables|Default|SetNewItemAmount 0)
            (Default|UpdateInventory _inventoryuiref self)))
        (elif (Utilities|Array|IsEmpty (Variables|Default|GetBaseItem))
          ;[0.15 0.15 0.15 0.5] Adding Item to Array
          (Utilities|Array|Add (Variables|Default|GetBaseItem) (Variables|/Game/BP_Master-Interactible.BP_Master-Interactible_C|GetBaseItemStruct (LocalVariables|GetL%20ItemInteracted)) :!label _label_3)
          (goto _label_2)
          (else
            ;[0.15 0.15 0.15 0.5] Checking Weapon
            (CallFunction|WeaponCheck (Variables|Default|GetBaseItem) (Variables|/Game/BP_Master-Interactible.BP_Master-Interactible_C|GetBaseItemStruct (LocalVariables|GetL%20ItemInteracted)))
            (if (Variables|Default|GetAddNew?)
              _
              (else
                (goto _label_3))))))
      ;[0.15 0.15 0.15 0.5] Destroy Item
      (Actor|DestroyActor (LocalVariables|GetL%20ItemInteracted))
      (return))))

(fn ShouldStackItem?
  (params (ItemFromInventory :type S%20Base%20Object%20Structure) (ItemFromCurrentActor :type S%20Base%20Object%20Structure))
  (bind (_inventoryitem_ _name _description _objecttype _mesh _icon _stackable_ _quantity) (Utilities|Struct|BreakS_BaseObject ItemFromInventory))
  (bind (_inventoryitem__2 _name_2 _description_2 _objecttype_2 _mesh_2 _icon_2 _stackable__2 _quantity_2 _maxquantity) (Utilities|Struct|BreakS_BaseObject ItemFromCurrentActor))
  (bind _returnvalue (+ _quantity _quantity_2))
  (bind _output_get (Variables|Default|SetFoundAndStackable? (Math|Boolean|ANDBoolean (Utilities|Enum|Equal(Enum) _name _name_2) _stackable__2 (<= _returnvalue _maxquantity) _inventoryitem__2)))
  (if _output_get
    (Variables|Default|SetNewItemAmount _returnvalue)
    (return true _returnvalue)
    (else
      (return false _quantity_2))))

(fn CheckItemType
  (params (From%20Invenytory :type S%20Base%20Object%20Structure) (ItemFromCurrentActor :type S%20Base%20Object%20Structure))
  (bind (_inventoryitem_ _name _description _objecttype) (Utilities|Struct|BreakS_BaseObject ItemFromCurrentActor))
  (return (and (Utilities|Enum|Equal(Enum) (.Name (Utilities|Struct|BreakS_BaseObject From%20Invenytory)) _name) (Utilities|Enum|Equal(Enum) _objecttype "NewEnumerator1"))))

(fn WeaponCheck
  (params (Array :type Array%20of%20S%20Base%20Object%20Structures) (ItemFromCurrentActor :type S%20Base%20Object%20Structure))
  (bind _array_element (Utilities|Array|ForEachLoopwithBreak Array :!label _label)
    (:LoopBody
      (bind _add_ (CallFunction|CheckItemType _array_element ItemFromCurrentActor))
      (bind _output_get (Variables|Default|SetAddNew? _add_))
      (if _output_get
        (goto _label Break)))))